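; BP_NiagaraIntruder is a static mesh actor that reports a food chain index, collision radius and world location, apparently as an intruder for Niagara-driven birds.
; The construction script applies the configured mesh, whose bounds supply the radius and location.
; When polled, the location getter picks a new random point within local bounds plus a Z offset every two seconds, using game-time modulo wraparound.
; Pickup and item physics hooks are empty.
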(event `/Game/BeefyBlackbirds/Blueprints/Interfaces/BPI_InteractiveObject.SetItemPhysics`
  (params (EnablePhysics :type Boolean) (InitialVelocity :type "Vector Structure")))

(fn `GetCollisionRadius`
  (returns (CollisionRadius :type "Float (double-precision)"))
  (return (`.SphereRadius` (`KismetSystemLibrary.GetComponentBounds` (`self.StaticMesh`)))))

(fn `GetFoodChainIndex`
  (returns (Index :type Integer))
  (return (`self.FoodChainIndex`)))

(fn `GetLocationWorldSpace`
  (returns (Location :type "Vector Structure"))
  (bind (_min _max) (`StaticMeshComponent.GetLocalBounds` (`self.StaticMesh`)))
  (`|ExecutionSequence`
    (:`then_0`
      (if (< (mod (`KismetSystemLibrary.GetGameTimeInSeconds`) 2.0) (`self.UpdateTimer`))
        (set `self.LocalFlightPointOffset` (+ (`KismetMathLibrary.MakeVector` (`KismetMathLibrary.Lerp` (.x _min) (.x _max) (`KismetMathLibrary.RandomFloat`)) (`KismetMathLibrary.Lerp` (.y _min) (.y _max) (`KismetMathLibrary.RandomFloat`)) (`KismetMathLibrary.Lerp` (.z _min) (.z _max) (`KismetMathLibrary.RandomFloat`))) (`KismetMathLibrary.MakeVector` 0.0 0.0 (`self.ParticleFlightPointOffsetZ`))))
        (set `self.UpdateTimer` 0.0)
        (else
          (set `self.UpdateTimer` (mod (`KismetSystemLibrary.GetGameTimeInSeconds`) 2.0)))))
    (:`then_1`
      (return (+ (`KismetSystemLibrary.GetComponentBounds` (`self.StaticMesh`)) (`self.LocalFlightPointOffset`))))))

(fn `PickupItem`
  (params (Location :type "Vector Structure") (Radius :type "Float (double-precision)") (CheckLocation :type Boolean))
  (returns (ItemClass :type "Actor Class Reference"))
  (return null))

(fn `UserConstructionScript`
  (`StaticMeshComponent.SetStaticMesh` (`self.StaticMesh`) (`self.Mesh`)))